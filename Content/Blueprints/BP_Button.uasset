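; BP_Button is a trigger button that changes color and signals a referenced door to open when overlapped.
; The construction script creates a dynamic material instance on the Button component and applies the main color.
; Any overlap with the Trigger component sets the highlighted color and calls OpenDoorMessage on DoorRef, with no filtering or reset logic.
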(event `self.Trigger.OnComponentBeginOverlap`
  (params (OverlappedComponent :type "PrimitiveComponent Object Reference") (OtherActor :type "Actor Object Reference") (OtherComp :type "PrimitiveComponent Object Reference") (OtherBodyIndex :type Integer) (bFromSweep :type Boolean) (SweepResult :type "HitResult Structure (by ref)"))
  (`MaterialInstanceDynamic.SetVectorParameterValue` (`self.DynMatInst`) "Color" (`self.HighlightedColor`))
  (message `/Game/Blueprints/BPI_Trigger.OpenDoor` (`self.DoorRef`)))

(fn `UserConstructionScript`
  (bind _returnvalue (`PrimitiveComponent.CreateDynamicMaterialInstance` (`self.Button`) 0 "/Game/Blueprints/Mat1_Inst.Mat1_Inst" "None"))
  (bind _output_get (set `self.DynMatInst` _returnvalue))
  (`MaterialInstanceDynamic.SetVectorParameterValue` _output_get "Color" (`self.MainColor`)))