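; BP_Platform is a platform that, when CanDisapear is set, repeatedly vanishes and reappears after an initial start delay.
; The construction script sets the mesh, adds an instance and creates a dynamic material tinted by a Color parameter.
; A rate-scaled timeline drives the color's alpha, then visibility and collision switch off.
; After a delay both return at full alpha, and after another delay the cycle calls itself again.
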(event `self.ReceiveBeginPlay`
  (`KismetSystemLibrary.Delay` (`self.StartDelay`))
  (`|ExecutionSequence`
    (:`then_0`
      (if (`self.CanDisapear?`)
        (`self.Dissapear`)))))

(event `Dissapear`
  (bind (_colorvalues_r _colorvalues_g _colorvalues_b) (break `LinearColor` (`self.ColorValues`)))
  (bind (_colorvalues_r_2 _colorvalues_g_2 _colorvalues_b_2) (break `LinearColor` (`self.ColorValues`)))
  (`TimelineComponent.SetPlayRate` (`self.Timeline`) (/ 1.0 (`self.PlayRate`)))
  (bind (_direction _newtrack_0) (`Timeline|Timeline` :!via `PlayFromStart`)
    (:`Update`
      (bind _output_get (set `self.ColorValues` (make `LinearColor` _colorvalues_r_2 _colorvalues_g_2 _colorvalues_b_2 _newtrack_0)))
      (`MaterialInstanceDynamic.SetVectorParameterValue` (`self.DynMatREF`) "Color" _output_get))
    (:`Finished`
      (`self.Disapear`)
      (`KismetSystemLibrary.Delay` (`self.Dealy Appear`))
      (bind _output_get_2 (set `self.ColorValues` (make `LinearColor` _colorvalues_r _colorvalues_g _colorvalues_b 1.0)))
      (`MaterialInstanceDynamic.SetVectorParameterValue` (`self.DynMatREF`) "Color" _output_get_2)
      (`self.Appear`)
      (`KismetSystemLibrary.Delay` (`self.Dealy Dispear`))
      (`self.Dissapear`))))

(fn `Appear`
  (`PrimitiveComponent.SetCollisionEnabled` (`self.Plateform`) "QueryAndPhysics")
  (`SceneComponent.SetVisibility` (`self.Plateform`) true true)
  (return))

(fn `Delay`
  (set `self.ColorValues` (make `LinearColor` 0.0 0.0 0.0 1.0)))

(fn `Disapear`
  (`PrimitiveComponent.SetCollisionEnabled` (`self.Plateform`) "NoCollision")
  (`SceneComponent.SetVisibility` (`self.Plateform`) false true)
  (return))

(fn `UserConstructionScript`
  (`StaticMeshComponent.SetStaticMesh` (`self.Plateform`) (`self.New Mesh`))
  (bind _returnvalue (`PrimitiveComponent.CreateDynamicMaterialInstance` (`self.Plateform`) 0 (`self.Source Material`) "None"))
  (bind _output_get (set `self.DynMatREF` _returnvalue))
  (`PrimitiveComponent.SetMaterial` (`self.Plateform`) 0 _output_get)
  (`MaterialInstanceDynamic.SetVectorParameterValue` (`self.DynMatREF`) "Color" (`self.ColorValues`))
  (`InstancedStaticMeshComponent.AddInstance` (`self.Plateform`) (`self.Instance Transform`) false))