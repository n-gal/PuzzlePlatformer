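; BP_Door is a key-gated door that opens once it has received the required number of keys.
; The construction script creates a dynamic material on the door mesh and tints it with the main color.
; Each OpenDoor call decrements the remaining key count, and at zero (or on BeginPlay if none are required) MovingDoor runs.
; MovingDoor switches to the highlight color and raises the mesh along Z with a timeline-driven lerp.
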(event `self.ReceiveBeginPlay`
  (set `self.nbOfTotalKeys` (`self.Nb of key required`))
  (if (== (`self.Nb of key required`) 0)
    (`self.MovingDoor`)))

(event `self.ReceiveActorBeginOverlap`
  (params (OtherActor :type "Actor Object Reference")))

(event `/Game/Blueprints/BPI_Trigger.OpenDoor`
  (`/Engine/EditorBlueprintResources/StandardMacros.DecrementInt` (`self.Nb of key required`)
    (:`  `
      (if (== (`self.Nb of key required`) 0)
        (`self.MovingDoor`)))))

(event `MovingDoor`
  (`MaterialInstanceDynamic.SetVectorParameterValue` (`self.DynMatInst`) "Color" (`self.HighlightedColor`))
  (bind (_direction _alpha) (`Timeline|Timeline`)
    (:`Update`
      (`SceneComponent.K2_SetRelativeLocation` (`self.Door`) (`KismetMathLibrary.VLerp` (0.0 0.0 0.0) (0.0 0.0 800.0) _alpha) false false))))

(fn `UserConstructionScript`
  (bind _returnvalue (`PrimitiveComponent.CreateDynamicMaterialInstance` (`self.Door`) 0 "/Game/Blueprints/Mat1_Inst.Mat1_Inst" "None"))
  (bind _output_get (set `self.DynMatInst` _returnvalue))
  (`MaterialInstanceDynamic.SetVectorParameterValue` _output_get "Color" (`self.MainColor`)))