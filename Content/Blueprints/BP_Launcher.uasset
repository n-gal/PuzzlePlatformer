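; Launch pad that throws the player character along the direction of its Arrow component, which the construction script rotates to a configurable rotation.
; When the player overlaps the trigger, move input is ignored for a launch delay, then LaunchCharacter overrides their velocity using the arrow's forward vector and a launch strength.
; A ready flag blocks retriggering until a short cooldown after launch, with the model's material showing whether a jump is available.
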(event `self.ReceiveBeginPlay`
  (`PrimitiveComponent.SetMaterial` (`self.LauncherModel`) 0 (`self.ValidJumpMaterial`)))

(event `self.Trigger.OnComponentBeginOverlap`
  (params (OverlappedComponent :type "PrimitiveComponent Object Reference") (OtherActor :type "Actor Object Reference") (OtherComp :type "PrimitiveComponent Object Reference") (OtherBodyIndex :type Integer) (bFromSweep :type Boolean) (SweepResult :type "HitResult Structure (by ref)"))
  (bind _returnvalue (`GameplayStatics.GetPlayerController` 0))
  (if (== OtherActor (`GameplayStatics.GetPlayerCharacter` 0))
    (if (`self.ReadyToThrow`)
      (set `self.ReadyToThrow` false)
      (`PrimitiveComponent.SetMaterial` (`self.LauncherModel`) 0 (`self.InvalidJumpMaterial`))
      (`Controller.SetIgnoreMoveInput` _returnvalue true)
      (`KismetSystemLibrary.Delay` (`self.LaunchDelay`))
      (`Controller.SetIgnoreMoveInput` _returnvalue false)
      (`self.LaunchPlayer`)
      (`KismetSystemLibrary.Delay` 1.0)
      (set `self.ReadyToThrow` true)
      (`PrimitiveComponent.SetMaterial` (`self.LauncherModel`) 0 (`self.ValidJumpMaterial`)))))

(fn `LaunchPlayer`
  (`Character.LaunchCharacter` (`GameplayStatics.GetPlayerCharacter` 0) (* (`KismetMathLibrary.GetForwardVector` (`SceneComponent.K2_GetComponentRotation` (`self.Arrow`))) (`self.LaunchStrength`)) true true))

(fn `UserConstructionScript`
  (`SceneComponent.K2_SetRelativeRotation` (`self.Arrow`) (`self.New Rotation`) false false))